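; BP_Player is the player Blueprint that manages the on-screen UI for gameplay and death.
; On BeginPlay, a locally controlled instance adds the crosshair and base HUD widgets.
; While Died is true, Tick removes both, creates a lose menu each frame without a guard, and switches player 0 to UI-only input with a cursor.
; An unconnected graph branch would swap crosshair and scope widgets on WantsToZoom, but never runs.
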(event EventBeginPlay
  (if (Pawn|IsLocallyControlled)
    (bind _returnvalue (UserInterface|CreateWidget "/Game/UI/WBP_Crosshair.WBP_Crosshair_C"))
    (bind _output_get (Variables|Default|SetCrosshair _returnvalue))
    (UserInterface|Viewport|AddtoViewport _output_get 0)
    (bind _returnvalue_2 (UserInterface|CreateWidget "/Game/UI/WBP_Base.WBP_Base_C"))
    (bind _output_get_2 (Variables|Default|SetUIBase _returnvalue_2))
    (UserInterface|Viewport|AddtoViewport _output_get_2 0)))

(event EventTick
  (params (DeltaSeconds :type Float%20%28single-precision%29))
  (bind _returnvalue (Game|GetPlayerController 0))
  (if (Variables|Default|GetbDied)
    (Widget|RemovefromParent (Variables|Default|GetUIBase))
    (bind _returnvalue_2 (UserInterface|CreateWidget "/Game/UI/WBP_LoseMenu.WBP_LoseMenu_C" _returnvalue))
    (UserInterface|Viewport|AddtoViewport _returnvalue_2 0)
    (Variables|/Script/Engine.PlayerController|SetbShowMouseCursor _returnvalue true)
    (Input|SetInputModeUIOnly _returnvalue _returnvalue_2 "LockOnCapture")))

(fn ConstructionScript)