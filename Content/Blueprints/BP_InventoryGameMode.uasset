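; BP_InventoryGameMode is the game mode for an inventory stage that precedes the Battlefield map.
; On PostLogin the server registers each BP_SPlayerController in the SGameInstance ConnectedPlayers list and tells it to create its inventory UI.
; LaunchGame server-travels to Battlefield, then hides the cursor and sets game-only input for player controller 0 only.
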(event Custom|LaunchGame
  (bind _returnvalue (Game|GetPlayerController 0))
  (Development|ExecuteConsoleCommand "ServerTravel Battlefield" _returnvalue)
  (Variables|/Script/Engine.PlayerController|SetbShowMouseCursor _returnvalue false)
  (Input|SetInputModeGameOnly _returnvalue))

(event EventPostLogin
  (params (NewPlayer :type Player%20Controller%20Object%20Reference))
  (Networking|SwitchHasAuthority
    (:Authority
      (bind _asbp_splayer_controller (Utilities|Casting|CastToBP_SPlayerController NewPlayer))
      (Utilities|Array|Add (Variables|/Script/CoopGame.SGameInstance|GetConnectedPlayers (.AsSGame%20Instance (Utilities|Casting|CastToSGameInstance (Game|GetGameInstance)))) _asbp_splayer_controller)
      (Default|CreateInventoryUI _asbp_splayer_controller))))

(fn ConstructionScript)