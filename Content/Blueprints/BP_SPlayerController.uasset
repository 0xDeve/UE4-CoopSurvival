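; BP_SPlayerController is a player controller that manages the inventory and loading screens and records the player's weapon choice.
; It creates the inventory widget with game-and-UI input and a visible cursor, then swaps it for a loading widget.
; Weapon selection branches on authority: the server writes the chosen class to SPlayerState and prints a debug message, while clients forward it through ServerSelectWeapon.
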(event Custom|LoadingScreen
  (Widget|RemovefromParent (Variables|Default|GetInventoryRef))
  (bind _returnvalue (UserInterface|CreateWidget "/Game/UI/WBP_Loading.WBP_Loading_C"))
  (UserInterface|Viewport|AddtoViewport _returnvalue 0)
  (Variables|Default|SetbShowMouseCursor false))

(event Custom|ServerSelectWeapon
  (params (WeaponSelection :type S%20Base%20Weapon%20Class%20Reference))
  (CallFunction|SelectWeapon WeaponSelection))

(event Custom|SelectWeapon
  (params (SelectedWeapon :type S%20Base%20Weapon%20Class%20Reference))
  (Networking|SwitchHasAuthority
    (:Authority
      (bind _assplayer_state (Utilities|Casting|CastToSPlayerState (Variables|Default|GetPlayerState)))
      (bind _output_get (Variables|/Script/CoopGame.SPlayerState|SetWeaponSelected _assplayer_state SelectedWeapon))
      (Development|PrintString (Utilities|String|Append (Utilities|GetDisplayName _assplayer_state) " selects " (Utilities|GetClassDisplayName _output_get)) true true "(R=0.000000,G=0.660000,B=1.000000,A=1.000000)" 1e+01))
    (:Remote
      (CallFunction|ServerSelectWeapon SelectedWeapon))))

(event Custom|CreateInventoryUI
  (bind _returnvalue (UserInterface|CreateWidget "/Game/UI/WBP_Inventory.WBP_Inventory_C" self))
  (bind _output_get (Variables|Default|SetInventoryRef _returnvalue))
  (UserInterface|Viewport|AddtoViewport _output_get 0)
  (Input|SetInputModeGameandUI self (Variables|Default|GetInventoryRef) "DoNotLock" true)
  (Variables|Default|SetbShowMouseCursor true))

(fn ConstructionScript)