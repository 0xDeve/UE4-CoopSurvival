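; BP_Player is the player Blueprint that sets up the on-screen HUD for the locally controlled player.
; On BeginPlay it creates crosshair, health indicator and ammo indicator widgets and adds them to the viewport, keeping a reference only to the crosshair.
; An unconnected chain, which never runs, would swap the crosshair for a scope widget based on WantsToZoom.
; Tick and the construction script are empty.
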(event EventBeginPlay
  (if (Pawn|IsLocallyControlled)
    (bind _returnvalue (UserInterface|CreateWidget "/Game/UI/WBP_Crosshair.WBP_Crosshair_C"))
    (bind _output_get (Variables|Default|SetCrosshair _returnvalue))
    (UserInterface|Viewport|AddtoViewport _output_get 0)
    (bind _returnvalue_2 (UserInterface|CreateWidget "/Game/UI/WBP_HealthIndicator.WBP_HealthIndicator_C"))
    (UserInterface|Viewport|AddtoViewport _returnvalue_2 0)
    (bind _returnvalue_3 (UserInterface|CreateWidget "/Game/UI/WBP_AmmoIndicator.WBP_AmmoIndicator_C"))
    (UserInterface|Viewport|AddtoViewport _returnvalue_3 0)))

(event EventTick
  (params (DeltaSeconds :type Float%20%28single-precision%29)))

(fn ConstructionScript)